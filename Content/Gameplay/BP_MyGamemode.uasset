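; BP_MyGamemode is a game mode Blueprint that opens a WebSocket connection to a server when play begins.
; BeginPlay binds message, connected, closed and error handlers on the WebSocketGameInstanceSubsystem, then connects to ServerURL after a short delay.
; Each handler only prints to screen, with errors shown in red, so it acts as a basic connection and logging harness.
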(event `self.ReceiveBeginPlay`
  (bind _returnvalue (subsystem `WebSocketGameInstanceSubsystem`))
  (`|ExecutionSequence`
    (:`then_0`
      (add `WebSocketGameInstanceSubsystem.OnMessageReceived` _returnvalue (`|CreateDelegate` :!event `OnWsMessageReceived`)))
    (:`then_1`
      (add `WebSocketGameInstanceSubsystem.OnConnected` _returnvalue (`|CreateDelegate` :!event `onWsConnected`)))
    (:`then_2`
      (add `WebSocketGameInstanceSubsystem.OnClosed` _returnvalue (`|CreateDelegate` :!event `OnWsClosed`)))
    (:`then_3`
      (add `WebSocketGameInstanceSubsystem.OnError` _returnvalue (`|CreateDelegate` :!event `OnWsError`)))
    (:`then_4`
      (`KismetSystemLibrary.Delay` 1.0)
      (`WebSocketGameInstanceSubsystem.Connect` (subsystem `WebSocketGameInstanceSubsystem`) (`self.Server URL`)))))

(fn `OnWsClosed`
  (`KismetSystemLibrary.PrintString` "Closed"))

(fn `OnWsConnected`
  (`KismetSystemLibrary.PrintString` "Connected"))

(fn `OnWsError`
  (params (Error :type String))
  (`KismetSystemLibrary.PrintString` Error true true (struct :`R` 1.0 :`G` 0.144648 :`B` 0.124752 :`A` 1.0)))

(fn `OnWsMessageReceived`
  (params (Message :type String))
  (`KismetSystemLibrary.PrintString` (`KismetStringLibrary.Concat_StrStr` "msg: " Message)))

(fn `UserConstructionScript`)